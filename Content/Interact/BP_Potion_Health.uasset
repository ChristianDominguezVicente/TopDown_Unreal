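; BP_Potion_Health is an interactable health potion pickup that is always available to interact with.
; On Interact, it casts the interacting actor to BP_TopDownCharacter, adds its ItemType row name to that character's BP_AC_Inventory component and destroys itself.
; An unconnected chain that applies the item directly to the character with a debug print remains in the graph but never runs.
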(event `/Game/Interact/BP_I_Interactuable.Interact`
  (params (InteractActor :type "Actor Object Reference"))
  (bind (_itemtype_datatable _itemtype_rowname) (break `DataTableRowHandle` (`self.ItemType`)))
  (bind _asbp_top_down_character (cast `/Game/TopDown/Blueprints/BP_TopDownCharacter` InteractActor))
  (bind _returnvalue (`self.GetComponentByClass` _asbp_top_down_character "/Game/Inventory/BP_AC_Inventory.BP_AC_Inventory_C"))
  (`/Engine/EditorBlueprintResources/StandardMacros.IsValid` _returnvalue
    (:`Is Valid`
      (`/Game/Inventory/BP_AC_Inventory.AddToInventory` _returnvalue _itemtype_rowname)
      (`self.K2_DestroyActor`))))

(fn `CanInteract`
  (returns (CanInteract :type Boolean))
  (return true))

(fn `UserConstructionScript`)