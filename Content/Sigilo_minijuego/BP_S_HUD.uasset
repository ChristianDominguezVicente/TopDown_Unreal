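; BP_S_HUD is the UI controller for the stealth minigame (Sigilo_minijuego), handling the pause menu and end screen.
; BeginPlay creates the pause and end widgets, adding only the end widget to the viewport immediately.
; Pause toggles the game's paused state and shows or removes the pause menu, tracked by an IsPaused flag.
; PlayerKilled and PlayerWin events forward the outcome to the end widget.
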(event `self.ReceiveBeginPlay`
  (bind _returnvalue (`|CreateWidget` "/Game/Menus/BP_MenuPausa.BP_MenuPausa_C" (`self.GetOwningPlayerController`)))
  (set `self.Pausa` _returnvalue)
  (bind _returnvalue_2 (`|CreateWidget` "/Game/Menus/BP_Fin.BP_Fin_C" (`self.GetOwningPlayerController`)))
  (bind _output_get (set `self.Fin` _returnvalue_2))
  (`UserWidget.AddToViewport` _output_get 0))

(event `PlayerKilled`
  (`/Game/Menus/BP_Fin.PlayerKilled` (`self.Fin`)))

(event `PlayerWin`
  (`/Game/Menus/BP_Fin.PlayerWin` (`self.Fin`)))

(fn `Pause`
  (if (`self.IsPaused`)
    ;[1 1 1] Si esta pausado
    (`GameplayStatics.SetGamePaused` false)
    (`Widget.RemoveFromParent` (`self.Pausa`))
    (set `self.IsPaused` false)
    (else
      ;[1 1 1] Si no esta pausado
      (`GameplayStatics.SetGamePaused` true)
      (`UserWidget.AddToViewport` (`self.Pausa`) 0)
      (set `self.IsPaused` true))))

(fn `UserConstructionScript`)