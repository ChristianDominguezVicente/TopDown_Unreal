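; BP_SigiloEnemy is the patrolling enemy of the stealth minigame, killing the player through the HUD when its capsule overlaps the player character.
; AI perception of a Player-tagged actor sets blackboard keys; otherwise a timer starts that clears them after a delay.
; GetNextPoint cycles through points of interest for patrol locations, falling back to its own location, and UpdateSpeed changes walk speed.
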(event `self.CapsuleComponent.OnComponentBeginOverlap`
  (params (OverlappedComponent :type "PrimitiveComponent Object Reference") (OtherActor :type "Actor Object Reference") (OtherComp :type "PrimitiveComponent Object Reference") (OtherBodyIndex :type Integer) (bFromSweep :type Boolean) (SweepResult :type "HitResult Structure (by ref)"))
  (cast `/Game/Sigilo_minijuego/BP_SigiloCharacter` OtherActor)
  (bind _asbp_s_hud (cast `/Game/Sigilo_minijuego/BP_S_HUD` (`PlayerController.GetHUD` (`GameplayStatics.GetPlayerController` 0))))
  (`/Game/Sigilo_minijuego/BP_S_HUD.PlayerKilled` _asbp_s_hud))

(event `self.ReceiveActorBeginOverlap`
  (params (OtherActor :type "Actor Object Reference")))

(event `self.AIPerception.OnTargetPerceptionUpdated`
  (params (Actor :type "Actor Object Reference") (Stimulus :type "AIStimulus Structure"))
  (bind _returnvalue (`AIBlueprintHelperLibrary.GetBlackboard` null))
  (if (and (`self.ActorHasTag` Actor "Player") (`.bSuccessfullySensed` (break `AIStimulus` Stimulus)))
    (`KismetSystemLibrary.K2_ClearAndInvalidateTimerHandle` (`self.EnemyTimer`))
    (`BlackboardComponent.SetValueAsBool` _returnvalue (`self.SensePlayer`) true)
    (`BlackboardComponent.SetValueAsObject` _returnvalue (`self.EnemyActor`) Actor)
    (else
      (bind _returnvalue_2 (`KismetSystemLibrary.K2_SetTimerDelegate` (delegate `LosePlayerTimer`) (`self.SenseTimer`)))
      (set `self.EnemyTimer` _returnvalue_2))))

(event `LosePlayerTimer`
  (bind _returnvalue (`AIBlueprintHelperLibrary.GetBlackboard` null))
  (`BlackboardComponent.SetValueAsBool` _returnvalue (`self.SensePlayer`) false)
  (`BlackboardComponent.SetValueAsObject` _returnvalue (`self.EnemyActor`) null))

(fn `GetNextPoint`
  (returns (NewPosition :type "Vector Structure"))
  (bind _pointsofinterest (`self.PointsOfInterest`))
  (if (> (`KismetArrayLibrary.Array_Length` _pointsofinterest) 0)
    (bind _result (`/Engine/EditorBlueprintResources/StandardMacros.IncrementInt` (`self.CurrentPoint`))
      (:`  `
        (if (`KismetArrayLibrary.Array_IsValidIndex` _pointsofinterest _result)
          (return (`self.K2_GetActorLocation` (`|GetArrayItem` _pointsofinterest _result)))
          (else
            (bind _output_get (set `self.CurrentPoint` 0))
            (return (`self.K2_GetActorLocation` (`|GetArrayItem` (`self.PointsOfInterest`) _output_get)))))))
    (else
      (return (`self.K2_GetActorLocation`)))))

(fn `UpdateSpeed`
  (params (`New Walk Speed` :type "Float (double-precision)"))
  (set `CharacterMovementComponent.MaxWalkSpeed` `New Walk Speed` (`self.CharacterMovement`)))

(fn `UserConstructionScript`)