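; BP_NPC is a placeholder non-player character that takes part in turn-based combat and can be interacted with.
; On BeginPlay it registers itself as a combat player with BP_TurnBaseGameMode.
; StartTurn prints the NPC's name, waits through a short delay, then tells the game mode to end its turn without acting.
; CanInteract always returns true, and Interact only prints a debug message.
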(event `self.ReceiveBeginPlay`
  (bind _asbp_turn_base_game_mode (cast `/Game/TurnCombat/BP_TurnBaseGameMode` (`GameplayStatics.GetGameMode`)))
  (`/Game/TurnCombat/BP_TurnBaseGameMode.RegisterCombatPlayer` _asbp_turn_base_game_mode self))

(event `/Game/TurnCombat/BP_I_CombatPlayer.StartTurn`
  (`KismetSystemLibrary.PrintString` (`KismetStringLibrary.Concat_StrStr` "Turn on" (`KismetSystemLibrary.GetDisplayName` self)))
  (`KismetSystemLibrary.Delay` 2.5)
  (bind _asbp_turn_base_game_mode (cast `/Game/TurnCombat/BP_TurnBaseGameMode` (`GameplayStatics.GetGameMode`)))
  (`/Game/TurnCombat/BP_TurnBaseGameMode.EndTurn` _asbp_turn_base_game_mode self))

(event `/Game/Interact/BP_I_Interactuable.Interact`
  (params (InteractActor :type "Actor Object Reference"))
  (`KismetSystemLibrary.PrintString` "Interacting with NPC"))

(fn `CanInteract`
  (returns (CanInteract :type Boolean))
  (return true))

(fn `UserConstructionScript`)