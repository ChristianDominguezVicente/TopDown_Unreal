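; BP_NPC_Dialog is an NPC that opens dialog on the player's HUD and can complete a quest during it.
; StartDialog checks the talking actor's BP_AC_QuestManager for the configured MissionToComplete.
; If that quest is in progress, it shows a hardcoded Quest1 or Quest2 row depending on CanComplete, completing the quest in the latter case.
; Otherwise it shows the NPC's configured Dialog row through BP_DialogHUD.
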(event `/Game/Dialog/BP_I_Dialog.StartDialog`
  (params (ActorToTalk :type "Actor Object Reference"))
  (bind _returnvalue (`self.GetComponentByClass` ActorToTalk "/Game/Misions/BP_AC_QuestManager.BP_AC_QuestManager_C"))
  (bind (_dialog_datatable _dialog_rowname) (break `DataTableRowHandle` (`self.Dialog`)))
  (bind (_missiontocomplete_datatable _missiontocomplete_rowname) (break `DataTableRowHandle` (`self.MissionToComplete`)))
  (bind _asbp_dialog_hud (cast `/Game/Dialog/BP_DialogHUD` (`PlayerController.GetHUD` (`GameplayStatics.GetPlayerController` 0))))
  (`/Engine/EditorBlueprintResources/StandardMacros.IsValid` _missiontocomplete_datatable
    (:`Is Valid`
      (`/Engine/EditorBlueprintResources/StandardMacros.IsValid` _returnvalue
        (:`Is Valid`
          (if (`KismetArrayLibrary.Array_Contains` (`/Game/Misions/BP_AC_QuestManager.InProgress` _returnvalue) _missiontocomplete_rowname)
            (bind _result (`/Game/Misions/BP_AC_QuestManager.CanComplete` _returnvalue _missiontocomplete_rowname))
            (if _result
              (`/Game/Dialog/BP_DialogHUD.ShowDialog` _asbp_dialog_hud "Quest2")
              (`/Game/Misions/BP_AC_QuestManager.CompleteQuest` _returnvalue _missiontocomplete_rowname)
              (else
                (`/Game/Dialog/BP_DialogHUD.ShowDialog` _asbp_dialog_hud "Quest1")))
            (else
              (`/Game/Dialog/BP_DialogHUD.ShowDialog` _asbp_dialog_hud _dialog_rowname :!label _label))))
        (:`Is Not Valid`
          (goto _label))))
    (:`Is Not Valid`
      (goto _label))))

(fn `CanInteract`)

(fn `UserConstructionScript`)