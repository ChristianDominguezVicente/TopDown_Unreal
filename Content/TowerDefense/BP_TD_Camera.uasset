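; BP_TD_Camera is the tower defense camera Blueprint that also tracks the player's lives and relays on-screen messages.
; BeginPlay caches the tower defense GameMode and the first player controller's HUD.
; DamageActor removes one life per call, notifies the GameMode of player death at exactly zero, and clamps negative counts to zero.
; ShowText forwards timed text to the HUD.
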(event `self.ReceiveBeginPlay`
  (bind _asbp_td_game_mode (cast `/Game/TowerDefense/BP_TD_GameMode` (`GameplayStatics.GetGameMode`)))
  (set `self.GameMode` _asbp_td_game_mode)
  (bind _asbp_td_hud (cast `/Game/TowerDefense/UI/BP_TD_HUD` (`PlayerController.GetHUD` (`GameplayStatics.GetPlayerController` 0))))
  (set `self.HUD` _asbp_td_hud))

(event `DamageActor`
  ;[1 1 1] Evento para cada vez que recibe daño y comprobar si se muere
  (bind _output_get (set `self.LIfes` (- (`self.LIfes`) 1)))
  (if (== _output_get 0)
    (bind _asbp_td_game_mode (cast `/Game/TowerDefense/BP_TD_GameMode` (`GameplayStatics.GetGameMode`)))
    (`/Game/TowerDefense/BP_TD_GameMode.PlayerDead` _asbp_td_game_mode)
    (elif (< _output_get 0)
      (set `self.LIfes` 0))))

(fn `ShowText`
  (params (Text :type Text) (Time :type "Float (double-precision)"))
  (`/Game/TowerDefense/UI/BP_TD_HUD.ShowTextInfo` (`self.HUD`) Text Time))

(fn `UserConstructionScript`)