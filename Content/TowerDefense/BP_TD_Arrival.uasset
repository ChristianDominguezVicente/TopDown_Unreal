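; BP_TD_Arrival is the goal point in the tower defense game, where arriving enemies cost the player a life.
; On BeginPlay it caches the player character as BP_TD_Camera, which holds the Lifes counter.
; When a BP_TD_EnemyBase begins overlapping its Box component, the enemy is destroyed and Lifes drops by one.
; Reaching exactly zero calls PlayerDead on BP_TD_GameMode, and negative values are reset to zero.
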(event `self.ReceiveBeginPlay`
  (bind _asbp_td_camera (cast `/Game/TowerDefense/BP_TD_Camera` (`GameplayStatics.GetPlayerCharacter` 0)))
  (set `self.m_PlayerCharacter` _asbp_td_camera))

(event `self.Box.OnComponentBeginOverlap`
  (params (OverlappedComponent :type "PrimitiveComponent Object Reference") (OtherActor :type "Actor Object Reference") (OtherComp :type "PrimitiveComponent Object Reference") (OtherBodyIndex :type Integer) (bFromSweep :type Boolean) (SweepResult :type "HitResult Structure (by ref)"))
  (bind _m_playercharacter (`self.m_PlayerCharacter`))
  (bind _asbp_td_enemy_base (cast `/Game/TowerDefense/Enemies/BP_TD_EnemyBase` OtherActor))
  (`self.K2_DestroyActor` _asbp_td_enemy_base)
  (bind _output_get (set `/Game/TowerDefense/BP_TD_Camera.Lifes` (- (`/Game/TowerDefense/BP_TD_Camera.Lifes` _m_playercharacter) 1) _m_playercharacter))
  (if (== _output_get 0)
    (bind _asbp_td_game_mode (cast `/Game/TowerDefense/BP_TD_GameMode` (`GameplayStatics.GetGameMode`)))
    (`/Game/TowerDefense/BP_TD_GameMode.PlayerDead` _asbp_td_game_mode)
    (elif (< _output_get 0)
      (set `/Game/TowerDefense/BP_TD_Camera.Lifes` 0 _m_playercharacter))))

(fn `UserConstructionScript`)