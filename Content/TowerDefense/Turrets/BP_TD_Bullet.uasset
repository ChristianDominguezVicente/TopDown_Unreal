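; BP_TD_Bullet is a tower defense projectile that damages enemies on overlap.
; It moves along its forward vector each Tick at a fixed speed, setting its location directly without sweep.
; Overlapping a BP_TD_EnemyBase calls Impact with a fixed damage value and destroys the bullet, while other actors are ignored.
; A timer started on BeginPlay destroys it after a few seconds if it hits no enemy.
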(event `self.ReceiveBeginPlay`
  (`KismetSystemLibrary.K2_SetTimerDelegate` (delegate `Destroy`) 3.0))

(event `Destroy`
  (`self.K2_DestroyActor`))

(event `self.ReceiveActorBeginOverlap`
  (params (OtherActor :type "Actor Object Reference"))
  (bind _asbp_td_enemy_base (cast `/Game/TowerDefense/Enemies/BP_TD_EnemyBase` OtherActor))
  (`/Game/TowerDefense/Enemies/BP_TD_Enemy01.Impact` _asbp_td_enemy_base 10)
  (`self.K2_DestroyActor`))

(event `self.ReceiveTick`
  (params (DeltaSeconds :type "Float (single-precision)"))
  (`self.K2_SetActorLocation` (+ (`self.K2_GetActorLocation`) (* (* DeltaSeconds 1000.0) (`self.GetActorForwardVector`)))))

(fn `UserConstructionScript`)