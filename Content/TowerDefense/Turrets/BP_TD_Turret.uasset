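; BP_TD_Turret is a tower defense turret that fires automatically and can be destroyed.
; Tick updates a health bar widget and turns it toward the player camera, then spawns BP_TD_Bullet at the fire point, rate-limited by a CanFire flag and Delay.
; Firing has no target check and only runs when the health bar widget cast succeeds.
; DamageTurret subtracts life and, at zero or below, spawns an explosion and destroys the actor.
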(event `self.ReceiveTick`
  (params (DeltaSeconds :type "Float (single-precision)"))
  (bind _healthbar_widget (`self.HealthBar Widget`))
  (bind _asbp_td_health_bar (cast `/Game/TowerDefense/UI/BP_TD_HealthBar` (`WidgetComponent.GetWidget` (`self.HealthBar Widget`))))
  (`ProgressBar.SetPercent` (`/Game/TowerDefense/UI/BP_TD_HealthBar.HealthBar` _asbp_td_health_bar) (/ (`self.Life`) (`self.MaxHealth`)))
  (`SceneComponent.K2_SetWorldRotation` _healthbar_widget (`KismetMathLibrary.FindLookAtRotation` (`SceneComponent.K2_GetComponentLocation` _healthbar_widget) (`SceneComponent.K2_GetComponentLocation` (`PlayerCameraManager.TransformComponent` (`GameplayStatics.GetPlayerCameraManager` 0)))) false false)
  (if (`self.CanFire`)
    (set `self.CanFire` false)
    (`|SpawnActorFromClass` "/Game/TowerDefense/Turrets/BP_TD_Bullet.BP_TD_Bullet_C" (`SceneComponent.K2_GetComponentToWorld` (`self.FirePoint`)) "Undefined" "MultiplyWithRoot" null null)
    (`KismetSystemLibrary.Delay` (`self.FireTime`))
    (set `self.CanFire` true)))

(event `DamageTurret`
  (params (Damage :type Integer))
  (bind (_returnvalue_location _returnvalue_rotation _returnvalue_scale) (`KismetMathLibrary.BreakTransform` (`SceneComponent.K2_GetComponentToWorld` (`self.Cube`))))
  (bind _output_get (set `self.Life` (- (`self.Life`) Damage)))
  (if (<= _output_get 0)
    (`GameplayStatics.SpawnEmitterAtLocation` "/Game/StarterContent/Particles/P_Explosion.P_Explosion" _returnvalue_location _returnvalue_rotation _returnvalue_scale)
    (`self.K2_DestroyActor`)))

(fn `UserConstructionScript`)