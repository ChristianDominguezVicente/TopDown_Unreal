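; Base enemy for a tower defense game that walks toward a fixed X line, keeping its Y, with the move reissued by a looping timer.
; Overlapping a turret stops movement and deals a single hit.
; Tick updates a health bar widget and turns it toward the camera.
; Impact subtracts life; at zero it notifies listeners and the GameMode, awards coins, spawns an explosion and destroys itself.
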(event `self.ReceiveBeginPlay`
  (`KismetSystemLibrary.K2_SetTimerDelegate` (delegate `MoveTo`) 1.0 true))

(event `MoveTo`
  (bind (_returnvalue_x _returnvalue_y) (`KismetMathLibrary.BreakVector` (`self.K2_GetActorLocation` self)))
  (`SkeletalMeshComponent.PlayAnimation` (`self.Mesh`) "/Game/Characters/Mannequins/Animations/Manny/MM_Walk_Fwd.MM_Walk_Fwd" true)
  (`|AIMoveTo` self (`KismetMathLibrary.MakeVector` -1040.0 _returnvalue_y -0.5) null 5.0 true))

(event `self.ReceiveTick`
  (params (DeltaSeconds :type "Float (single-precision)"))
  (bind _healthbar_widget (`self.HealthBar Widget`))
  (bind _asbp_td_health_bar (cast `/Game/TowerDefense/UI/BP_TD_HealthBar` (`WidgetComponent.GetWidget` (`self.HealthBar Widget`))))
  (`ProgressBar.SetPercent` (`/Game/TowerDefense/UI/BP_TD_HealthBar.HealthBar` _asbp_td_health_bar) (/ (`self.Life`) (`self.MaxHealth`)))
  (`SceneComponent.K2_SetWorldRotation` _healthbar_widget (`KismetMathLibrary.FindLookAtRotation` (`SceneComponent.K2_GetComponentLocation` _healthbar_widget) (`SceneComponent.K2_GetComponentLocation` (`PlayerCameraManager.TransformComponent` (`GameplayStatics.GetPlayerCameraManager` 0)))) false false))

(event `LifeDecrease`
  (params (Damage :type Integer))
  (set `self.Life` (- (`self.Life`) Damage)))

(event `self.Box.OnComponentBeginOverlap`
  (params (OverlappedComponent :type "PrimitiveComponent Object Reference") (OtherActor :type "Actor Object Reference") (OtherComp :type "PrimitiveComponent Object Reference") (OtherBodyIndex :type Integer) (bFromSweep :type Boolean) (SweepResult :type "HitResult Structure (by ref)"))
  (bind _asbp_td_turret (cast `/Game/TowerDefense/Turrets/BP_TD_Turret` OtherActor))
  (`MovementComponent.StopMovementImmediately` (`self.CharacterMovement`))
  (`self.Attack` _asbp_td_turret))

(event `self.Box.OnComponentEndOverlap`
  (params (OverlappedComponent :type "PrimitiveComponent Object Reference") (OtherActor :type "Actor Object Reference") (OtherComp :type "PrimitiveComponent Object Reference") (OtherBodyIndex :type Integer))
  (cast `/Game/TowerDefense/Turrets/BP_TD_Turret` OtherActor
    (:`CastFailed`
      (`self.MoveTo`))))

(event `Impact`
  (params (NewParam :type Integer))
  (bind (_returnvalue_location _returnvalue_rotation _returnvalue_scale) (`KismetMathLibrary.BreakTransform` (`SceneComponent.K2_GetComponentToWorld` (`self.Mesh`))))
  (`self.LifeDecrease` NewParam)
  (if (<= (`self.Life`) 0)
    (`self.OnEnemyDestroy`)
    (bind _asbp_td_game_mode (cast `/Game/TowerDefense/BP_TD_GameMode` (`GameplayStatics.GetGameMode`)))
    (`/Game/TowerDefense/BP_TD_GameMode.EnemyDestroyed` _asbp_td_game_mode)
    (`/Game/TowerDefense/BP_TD_GameMode.AddCoins` _asbp_td_game_mode (`self.Coins`))
    (`GameplayStatics.SpawnEmitterAtLocation` "/Game/StarterContent/Particles/P_Explosion.P_Explosion" _returnvalue_location _returnvalue_rotation _returnvalue_scale)
    (`self.K2_DestroyActor`)))

(fn `Attack`
  (params (Turret :type "/Game/TowerDefense/Turrets/BP_TD_Turret Object Reference"))
  (`/Game/TowerDefense/Turrets/BP_TD_Turret.DamageTurret` Turret 5))

(fn `UserConstructionScript`)