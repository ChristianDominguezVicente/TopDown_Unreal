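; Tower defense enemy generator that spawns random AI enemies on a looping timer.
; Each spawn picks a random SpawnPoint-tagged component and one of three enemy classes, with the random range set by the game mode's Level and clamped by MaxNumEnemies.
; Each enemy's destroy event decrements SpawnTime, but the timer is never reset, so its interval stays unchanged.
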(event `self.ReceiveBeginPlay`
  (`KismetSystemLibrary.K2_SetTimerDelegate` (delegate `Spawn`) (`self.SpawnTime`) true)
  (bind _asbp_td_game_mode (cast `/Game/TowerDefense/BP_TD_GameMode` (`GameplayStatics.GetGameMode`)))
  (set `self.m_GameMode` _asbp_td_game_mode))

(event `Spawn`
  (bind _enemyspawn (`self.SpawnEnemy`))
  (bind _asbp_td_enemy_base (cast `/Game/TowerDefense/Enemies/BP_TD_EnemyBase` _enemyspawn))
  (add `/Game/TowerDefense/Enemies/BP_TD_EnemyBase.OnEnemyDestroy` _asbp_td_enemy_base (delegate `EnemyDestroyed`)))

(event `EnemyDestroyed`
  (set `self.SpawnTime` (- (`self.SpawnTime`) 1.0)))

(fn `GetClassToSpawn`
  (params (Type :type Integer))
  (returns (Class :type "/Game/TowerDefense/Enemies/BP_TD_EnemyBase Class Reference"))
  (return (select `int` (`KismetMathLibrary.Clamp` Type 0 (- (`self.MaxNumEnemies`) 1)) :`0` "/Game/TowerDefense/Enemies/BP_TD_Enemy01.BP_TD_Enemy01_C" :`1` "/Game/TowerDefense/Enemies/BP_TD_Enemy02.BP_TD_Enemy02_C" :`2` "/Game/TowerDefense/Enemies/BP_TD_Enemy03.BP_TD_Enemy03_C" :!type "/Game/TowerDefense/Enemies/BP_TD_EnemyBase Class Reference")))

(fn `SpawnEnemy`
  (returns (EnemySpawn :type "/Game/TowerDefense/Enemies/BP_TD_EnemyBase Object Reference"))
  (bind _returnvalue (`self.GetComponentsByTag` "/Script/Engine.SceneComponent" "SpawnPoint"))
  (bind _class (`self.GetClassToSpawn` (`KismetMathLibrary.RandomInteger` (`/Game/TowerDefense/BP_TD_GameMode.Level` (`self.m_GameMode`)))))
  (bind _returnvalue_2 (`AIBlueprintHelperLibrary.SpawnAIFromClass` _class null (`SceneComponent.K2_GetComponentLocation` (`|GetArrayItem` _returnvalue (`KismetMathLibrary.RandomInteger` (`KismetArrayLibrary.Array_Length` _returnvalue)))) (struct :`Yaw` 180.0) false null))
  (bind _asbp_td_enemy_base (cast `/Game/TowerDefense/Enemies/BP_TD_EnemyBase` _returnvalue_2))
  (return _asbp_td_enemy_base))

(fn `UserConstructionScript`)