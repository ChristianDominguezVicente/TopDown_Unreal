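; BP_NPC_RPG is the enemy combatant in a turn-based combat game, showing its HP on the TurnHUD.
; On StartTurn it sets the HUD turn label, faces the player, fires an EnemyBullet from its spawn point, then after a fixed delay tells BP_TurnBaseGameMode to end its turn.
; TakeDamage reduces HP, refreshes the HUD, and at zero or below destroys the actor and triggers the player win screen.
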(event `self.ReceiveBeginPlay`
  (`parent.ReceiveBeginPlay`)
  (bind _asturn_hud (cast `/Game/TurnCombat/TurnHUD` (`PlayerController.GetHUD` (`GameplayStatics.GetPlayerController` 0))))
  (`/Game/TurnCombat/TurnHUD.SetEnemyHp` _asturn_hud (`KismetTextLibrary.Conv_StringToText` (`KismetStringLibrary.Concat_StrStr` "Enemy HP: " (`KismetStringLibrary.Conv_DoubleToString` (`self.HP`))))))

(event `self.ReceiveTick`
  (params (DeltaSeconds :type "Float (single-precision)"))
  (`parent.ReceiveTick` DeltaSeconds))

(event `/Game/TurnCombat/BP_I_CombatPlayer.StartTurn`
  (bind _asturn_hud (cast `/Game/TurnCombat/TurnHUD` (`PlayerController.GetHUD` (`GameplayStatics.GetPlayerController` 0))))
  (`/Game/TurnCombat/TurnHUD.SetTurn` _asturn_hud "Enemy Turn")
  (`self.K2_SetActorRotation` (`KismetMathLibrary.FindLookAtRotation` (`self.K2_GetActorLocation`) (`self.K2_GetActorLocation` (`GameplayStatics.GetPlayerCharacter` 0))))
  (bind _returnvalue (`|SpawnActorFromClass` "/Game/TurnCombat/EnemyBullet.EnemyBullet_C" (`SceneComponent.K2_GetComponentToWorld` (`self.SpwnPoint`)) "Undefined" "MultiplyWithRoot" null null))
  (`self.K2_SetActorRotation` _returnvalue (`self.K2_GetActorRotation`) false)
  (`KismetSystemLibrary.Delay` 2.5)
  (bind _asbp_turn_base_game_mode (cast `/Game/TurnCombat/BP_TurnBaseGameMode` (`GameplayStatics.GetGameMode`)))
  (`/Game/TurnCombat/BP_TurnBaseGameMode.EndTurn` _asbp_turn_base_game_mode self))

(fn `TakeDamage`
  (params (Damage :type "Float (double-precision)"))
  (bind _output_get (set `self.HP` (- (`self.HP`) Damage)))
  (bind _asturn_hud (cast `/Game/TurnCombat/TurnHUD` (`PlayerController.GetHUD` (`GameplayStatics.GetPlayerController` 0))))
  (`/Game/TurnCombat/TurnHUD.SetEnemyHp` _asturn_hud (`KismetTextLibrary.Conv_StringToText` (`KismetStringLibrary.Concat_StrStr` "Enemy HP: " (`KismetStringLibrary.Conv_DoubleToString` (`self.HP`)))))
  (if (<= _output_get 0.0)
    (`self.K2_DestroyActor`)
    (bind _asturn_hud_2 (cast `/Game/TurnCombat/TurnHUD` (`PlayerController.GetHUD` (`GameplayStatics.GetPlayerController` 0))))
    (`/Game/TurnCombat/TurnHUD.PlayerWin` _asturn_hud_2)))

(fn `UserConstructionScript`
  (`parent.UserConstructionScript`))