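; Turn-based combat game mode that keeps a list of combat actors and decides who acts next.
; The player character is added on BeginPlay, and other combatants register or unregister through events.
; StartCombat and EndTurn pick a random actor other than the last one and send it a start-turn message.
; When one or fewer combatants remain at the end of a turn, it reports combat as ended.
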(event `self.ReceiveBeginPlay`
  (bind _asbp_i_combat_player (cast `/Game/TurnCombat/BP_I_CombatPlayer` (`GameplayStatics.GetPlayerCharacter` 0)))
  (`KismetArrayLibrary.Array_AddUnique` (`self.CombatActors`) _asbp_i_combat_player))

(event `RegisterCombatPlayer`
  (params (Actor :type "/Game/TurnCombat/BP_I_CombatPlayer Interface"))
  (`KismetArrayLibrary.Array_AddUnique` (`self.CombatActors`) Actor))

(event `UnregisterCombatPlayer`
  (params (Actor :type "/Game/TurnCombat/BP_I_CombatPlayer Interface"))
  (`KismetArrayLibrary.Array_RemoveItem` (`self.CombatActors`) Actor))

(event `StartCombat`
  (`KismetSystemLibrary.PrintString` "Start Combat" true true (struct :`R` 1.0 :`G` 1.0 :`B` 1.0 :`A` 1.0))
  (bind _index (`self.SelectNextTurn` null))
  (message `/Game/TurnCombat/BP_I_CombatPlayer.StartTurn` (`KismetSystemLibrary.Conv_InterfaceToObject` (`|GetArrayItem` (`self.CombatActors`) _index))))

(event `EndTurn`
  (params (Actor :type "/Game/TurnCombat/BP_I_CombatPlayer Interface"))
  (if (> (`KismetArrayLibrary.Array_Length` (`self.CombatActors`)) 1)
    (bind _index (`self.SelectNextTurn` Actor))
    (message `/Game/TurnCombat/BP_I_CombatPlayer.StartTurn` (`KismetSystemLibrary.Conv_InterfaceToObject` (`|GetArrayItem` (`self.CombatActors`) _index)))
    (else
      (`KismetSystemLibrary.PrintString` "Combat Ended"))))

(fn `SelectNextTurn`
  (params (LastCombat :type "/Game/TurnCombat/BP_I_CombatPlayer Interface"))
  (returns (Index :type Integer))
  (locals (LastIndex :type Integer :default 0) (Found :type Boolean) (FoundIndex :type Integer))
  (bind _combatactors (`self.CombatActors`))
  (set `local.LastIndex` (`KismetArrayLibrary.Array_Find` _combatactors LastCombat))
  (while (not (`local.Found`))
    (set `local.FoundIndex` (`KismetMathLibrary.RandomInteger` (`KismetArrayLibrary.Array_Length` _combatactors)))
    (if (!= (`local.FoundIndex`) (`local.LastIndex`))
      (set `local.Found` true)))
  (return (`local.FoundIndex`)))

(fn `UserConstructionScript`)