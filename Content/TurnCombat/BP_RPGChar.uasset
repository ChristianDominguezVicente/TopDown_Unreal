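; Player character for turn-based RPG combat, able to move and make one attack during each timed turn.
; StartTurn enables input and movement, then after a fixed delay notifies BP_TurnBaseGameMode, locks control and re-arms the attack.
; Space plays an explosion effect and runs a debug-drawn forward capsule trace that damages a hit BP_NPC_RPG.
; GetDamage lowers HP, refreshes TurnHUD and reports player death at zero.
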(event `self.ReceiveBeginPlay`
  (`parent.ReceiveBeginPlay`)
  (bind _asturn_hud (cast `/Game/TurnCombat/TurnHUD` (`PlayerController.GetHUD` (`GameplayStatics.GetPlayerController` 0))))
  (`/Game/TurnCombat/TurnHUD.SetPlayerHp` _asturn_hud (`KismetTextLibrary.Conv_StringToText` (`KismetStringLibrary.Concat_StrStr` "Player HP: " (`KismetStringLibrary.Conv_DoubleToString` (`self.HP`))))))

(event `Key|SpaceBar`
  (params (Key :type "Key Structure"))
  (:`Pressed`
    (`self.Attack`)))

(event `/Game/TurnCombat/BP_I_CombatPlayer.StartTurn`
  (set `self.canMove` true)
  (bind _asturn_hud (cast `/Game/TurnCombat/TurnHUD` (`PlayerController.GetHUD` (`GameplayStatics.GetPlayerController` 0))))
  (`/Game/TurnCombat/TurnHUD.SetTurn` _asturn_hud "Player Turn")
  (`self.EnableInput` (`GameplayStatics.GetPlayerController` 0) null)
  (`KismetSystemLibrary.Delay` 6.0)
  (bind _asbp_turn_base_game_mode (cast `/Game/TurnCombat/BP_TurnBaseGameMode` (`GameplayStatics.GetGameMode`)))
  (`/Game/TurnCombat/BP_TurnBaseGameMode.EndTurn` _asbp_turn_base_game_mode self)
  (set `self.canMove` false)
  (`self.DisableInput` (`GameplayStatics.GetPlayerController` 0) null)
  (set `self.canAttack` true))

(fn `Attack`
  (bind _returnvalue (`self.K2_GetActorLocation`))
  (bind _returnvalue_2 (+ _returnvalue (* (`self.GetActorForwardVector`) 100.0)))
  (if (`self.canMove`)
    (if (`self.canAttack`)
      (`GameplayStatics.SpawnEmitterAtLocation` "/Game/StarterContent/Particles/P_Explosion.P_Explosion" _returnvalue_2)
      (`GameplayStatics.PlaySound2D` "/Game/StarterContent/Audio/Explosion01.Explosion01" 1.0 1.0 0.0 null null)
      (bind _outhit (`KismetSystemLibrary.CapsuleTraceSingle` :`Start` _returnvalue :`End` _returnvalue_2 :`Radius` 100.0 :`HalfHeight` 100.0 :`TraceChannel` "TraceTypeQuery3" :`DrawDebugType` "ForDuration" :`DrawTime` 15.0))
      (bind _asbp_npc_rpg (cast `/Game/TurnCombat/BP_NPC_RPG` (`.HitActor` (`GameplayStatics.BreakHitResult` _outhit))))
      (`/Game/TurnCombat/BP_NPC_RPG.TakeDamage` _asbp_npc_rpg 2.0)
      (set `self.canAttack` false))))

(fn `GetDamage`
  (params (Damage :type "Float (double-precision)"))
  (set `self.HP` (- (`self.HP`) Damage))
  (bind _asturn_hud (cast `/Game/TurnCombat/TurnHUD` (`PlayerController.GetHUD` (`GameplayStatics.GetPlayerController` 0))))
  (`/Game/TurnCombat/TurnHUD.SetPlayerHp` _asturn_hud (`KismetTextLibrary.Conv_StringToText` (`KismetStringLibrary.Concat_StrStr` "Player HP: " (`KismetStringLibrary.Conv_DoubleToString` (`self.HP`)))))
  (if (<= (`self.HP`) 0.0)
    (bind _asturn_hud_2 (cast `/Game/TurnCombat/TurnHUD` (`PlayerController.GetHUD` (`GameplayStatics.GetPlayerController` 0))))
    (`/Game/TurnCombat/TurnHUD.PlayerKilled` _asturn_hud_2)))

(fn `Move`
  (if (`self.canMove`)
    (`parent.Move`)))

(fn `UserConstructionScript`
  (`parent.UserConstructionScript`))