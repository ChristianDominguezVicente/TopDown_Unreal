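; Quest manager component that tracks the in-progress and completed quests of its owning actor.
; StartQuest and CompleteQuest update those lists and refresh the quest display on SDI_BP_HUD.
; CanComplete reads the Quests data table: Objects quests count matching items in the owner's BP_SDI_Inventory against a required value.
; Talk quests always return false, as their related-quest check is disconnected.
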(fn `CanComplete`
  (params (ID :type Name))
  (returns (Result :type Boolean))
  (locals (CanComplete :type Boolean) (NumberOfObjects :type Integer))
  (bind _returnvalue (`Actor.GetComponentByClass` (`self.GetOwner`) "/Game/DialogInventoryLevel/BP_SDI_Inventory/BP_SDI_Inventory.BP_SDI_Inventory_C"))
  (bind _returnvalue_2 (`|GetDataTableRow` (`self.Quests`) ID)
    (:`then`
      (bind (_name _description _type _relatedquests _value _objectname) (break `/Game/Misions/F_Quest` _returnvalue_2))
      (switch `/Game/Misions/E_QuestType` _type
        (:`NewEnumerator0`
          ;[1 1 1] Talk logic
          ; If there is no related tasks to complete can be completed
          ; If not, check realted task are completed
          (set `local.CanComplete` false)
          (return (`local.CanComplete`)))
        (:`NewEnumerator2`
          ;[1 1 1] Check objects in inventory
          (`/Engine/EditorBlueprintResources/StandardMacros.IsValid` _returnvalue
            (:`Is Valid`
              (set `local.NumberOfObjects` 0)
              (for _array_element (`/Game/DialogInventoryLevel/BP_SDI_Inventory/BP_SDI_Inventory.Inventory` _returnvalue)
                (if (== _array_element _objectname)
                  (`/Engine/EditorBlueprintResources/StandardMacros.IncrementInt` (`local.NumberOfObjects`))))
              (return (>= (`local.NumberOfObjects`) _value)))))))
    (:`RowNotFound`
      (return false))))

(fn `CompleteQuest`
  (params (ID :type Name))
  (`KismetArrayLibrary.Array_RemoveItem` (`self.InProgress`) ID)
  (`KismetArrayLibrary.Array_AddUnique` (`self.Completed`) ID)
  (bind _assdi_bp_hud (cast `/Game/DialogInventoryLevel/BP_SDI_Dialog/SDI_BP_HUD` (`PlayerController.GetHUD` (`GameplayStatics.GetPlayerController` 0))))
  (`/Game/DialogInventoryLevel/BP_SDI_Dialog/SDI_BP_HUD.UpdateQuests` _assdi_bp_hud))

(fn `StartQuest`
  (params (ID :type Name))
  (if (!= ID "None")
    (`KismetArrayLibrary.Array_AddUnique` (`self.InProgress`) ID)
    (bind _assdi_bp_hud (cast `/Game/DialogInventoryLevel/BP_SDI_Dialog/SDI_BP_HUD` (`PlayerController.GetHUD` (`GameplayStatics.GetPlayerController` 0))))
    (`/Game/DialogInventoryLevel/BP_SDI_Dialog/SDI_BP_HUD.UpdateQuests` _assdi_bp_hud)))