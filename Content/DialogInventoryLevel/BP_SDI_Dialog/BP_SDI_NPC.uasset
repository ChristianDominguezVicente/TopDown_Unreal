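; Dialog and quest NPC for the SDI system that shows its name and opens HUD dialog when StartDialog is called.
; If the talking actor's BP_SDI_QuestManager has MissionToComplete in progress, it shows a quest-specific dialog and completes the quest when possible.
; Otherwise it shows the default Dialog row.
; FindQuest hardcodes dialog row names for missions MS2 and MS3, chosen by whether the quest can be completed.
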(event `self.ReceiveBeginPlay`
  ;[1 1 1] Name NPC
  (`TextRenderComponent.K2_SetText` (`self.NameNPC`) (`KismetTextLibrary.Conv_StringToText` (`self.NPCName`))))

(event `/Game/Dialog/BP_I_Dialog.StartDialog`
  (params (ActorToTalk :type "Actor Object Reference"))
  (bind _returnvalue (`self.GetComponentByClass` ActorToTalk "/Game/DialogInventoryLevel/BP_SDI_Missions/BP_SDI_QuestManager.BP_SDI_QuestManager_C"))
  (bind (_dialog_datatable _dialog_rowname) (break `DataTableRowHandle` (`self.Dialog`)))
  (bind (_missiontocomplete_datatable _missiontocomplete_rowname) (break `DataTableRowHandle` (`self.MissionToComplete`)))
  (set `self.QuestCompleted` false)
  (bind _assdi_bp_hud (cast `/Game/DialogInventoryLevel/BP_SDI_Dialog/SDI_BP_HUD` (`PlayerController.GetHUD` (`GameplayStatics.GetPlayerController` 0))))
  (`/Engine/EditorBlueprintResources/StandardMacros.IsValid` _missiontocomplete_datatable
    (:`Is Valid`
      (`/Engine/EditorBlueprintResources/StandardMacros.IsValid` _returnvalue
        (:`Is Valid`
          (if (`KismetArrayLibrary.Array_Contains` (`/Game/DialogInventoryLevel/BP_SDI_Missions/BP_SDI_QuestManager.InProgress` _returnvalue) _missiontocomplete_rowname)
            ;[1 1 1] complete and show dialog
            (bind _result (`/Game/DialogInventoryLevel/BP_SDI_Missions/BP_SDI_QuestManager.CanComplete` _returnvalue _missiontocomplete_rowname))
            (bind _namedialog (`self.FindQuest` _result))
            (`/Game/DialogInventoryLevel/BP_SDI_Dialog/SDI_BP_HUD.ShowDialog` _assdi_bp_hud _namedialog)
            (if _result
              (`/Game/DialogInventoryLevel/BP_SDI_Missions/BP_SDI_QuestManager.CompleteQuest` _returnvalue _missiontocomplete_rowname)
              (set `self.QuestCompleted` true))
            (else
              (`/Game/DialogInventoryLevel/BP_SDI_Dialog/SDI_BP_HUD.ShowDialog` _assdi_bp_hud _dialog_rowname :!label _label))))
        (:`Is Not Valid`
          (goto _label))))
    (:`Is Not Valid`
      (goto _label))))

(fn `CanInteract`)

(fn `FindQuest`
  (params (CanComplete :type Boolean))
  (returns (NameDialog :type Name))
  (locals (CanCompleteMS :type Boolean))
  (bind (_missiontocomplete_datatable _missiontocomplete_rowname) (break `DataTableRowHandle` (`self.MissionToComplete`)))
  (bind _output_get (set `local.CanCompleteMS` CanComplete))
  ;[1 1 1] mission ms2
  (if (== _missiontocomplete_rowname "MS2")
    (if _output_get
      (set `self.Quest Name` "Quest2")
      (else
        (set `self.Quest Name` "Quest1")))
    (return (`self.Quest Name`))
    (else
      ;[1 1 1] mission ms3
      (if (== _missiontocomplete_rowname "MS3")
        (if (`local.CanCompleteMS`)
          (set `self.Quest Name` "Chest1")
          (else
            (set `self.Quest Name` "Chest2")))
        (return (`self.Quest Name`))))))

(fn `UserConstructionScript`)